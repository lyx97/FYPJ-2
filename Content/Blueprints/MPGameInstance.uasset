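; Game instance Blueprint that manages LAN multiplayer sessions through events to host, search, join and destroy games.
; Hosting creates a session with zero public connections, then opens FirstPersonExampleMap as a listen server via console command.
; Searching stores the found sessions in SessionResult, and joining uses its first entry without a bounds check.
; Each operation prints debug status text, except a successful search.
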(event `HOSTGame`
  ;[1 1 1] HOST GAME
  (`CreateSessionCallbackProxy.CreateSession` (`GameplayStatics.GetPlayerController` 0) 0 true
    (:`OnSuccess`
      (`KismetSystemLibrary.ExecuteConsoleCommand` "open FirstPersonExampleMap?listen")
      (`KismetSystemLibrary.PrintString` "GAME CREATED"))
    (:`OnFailure`
      (`KismetSystemLibrary.PrintString` "GAME FAILED TO CREATE"))))

(event `SEARCHGame`
  ;[1 1 1] SEARCH GAME
  (bind _results (`FindSessionsCallbackProxy.FindSessions` (`GameplayStatics.GetPlayerController` 0) 2 true)
    (:`OnSuccess`
      (set `self.SessionResult` _results))
    (:`OnFailure`
      (`KismetSystemLibrary.PrintString` "CANNOT FIND GAME"))))

(event `JOINGame`
  ;[1 1 1] JOIN GAME
  (`JoinSessionCallbackProxy.JoinSession` (`GameplayStatics.GetPlayerController` 0) (`|GetArrayItem` (`self.SessionResult`))
    (:`OnSuccess`
      (`KismetSystemLibrary.PrintString` "JOINED GAME"))
    (:`OnFailure`
      (`KismetSystemLibrary.PrintString` "FAILED TO JOIN GAME"))))

(event `DESTROYGame`
  ;[1 1 1] DESTROY GAME
  (`DestroySessionCallbackProxy.DestroySession` (`GameplayStatics.GetPlayerController` 0)
    (:`OnSuccess`
      (`KismetSystemLibrary.PrintString` "GAME REMOVED"))
    (:`OnFailure`
      (`KismetSystemLibrary.PrintString` "FAILED TO REMOVE GAME"))))