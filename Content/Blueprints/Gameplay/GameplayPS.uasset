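; GameplayPS is a player state that relays in-game chat messages between players.
; With authority, BroadcastChatMessage loops over the game state's PlayerArray and calls BroadcastChatMessageMulticast on each GameplayPS.
; The sender label combines the owning GameplayPC's saved player name with PlayerName in parentheses, noted as being for Steam.
; Each multicast event fires the ReceiveChatMessageGameplay dispatcher with sender and message.
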(event `BroadcastChatMessage`
  (params (ChatMessageIn :type Text))
  ;[1 1 1] Handle chat message, broadcasting and receiving
  (`/Engine/EditorBlueprintResources/ActorMacros.Switch Has Authority`
    (:`Authority`
      (for _array_element (`GameStateBase.PlayerArray` (`GameplayStatics.GetGameState`))
        (bind _asgameplay_ps (cast `/Game/Blueprints/Gameplay/GameplayPS` _array_element))
        (`self.BroadcastChatMessageMulticast` _asgameplay_ps (`KismetTextLibrary.Conv_StringToText` (`KismetStringLibrary.Concat_StrStr` (`KismetTextLibrary.Conv_TextToString` (`.MyPlayerName_2_D9D1EF88454FFEE914685A9CBAF41908` (break `/Game/Blueprints/AllLevels/PlayerInfo` (`/Game/Blueprints/Gameplay/GameplayPC.PlayerSettings` (cast `/Game/Blueprints/Gameplay/GameplayPC` (`self.GetOwner`) :!pure true))))) " (" (`self.PlayerName`) ")")) ChatMessageIn)))))

(event `BroadcastChatMessageMulticast`
  (params (ChatSender :type Text) (ChatMessageIn :type Text))
  ;[1 1 1] Handle chat message, broadcasting and receiving
  (`self.ReceiveChatMessageGameplay` ChatSender ChatMessageIn))

(fn `UserConstructionScript`)