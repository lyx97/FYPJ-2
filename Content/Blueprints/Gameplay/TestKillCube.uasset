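; Test cube actor that takes damage and destroys itself once its health runs out.
; TakeDamage passes through an authority switch with no branch-specific logic, then calls ApplyDamage to subtract the damage from Health.
; Tick polls Health every frame and destroys the actor when it reaches zero or below.
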(event `self.ReceiveTick`
  (params (DeltaSeconds :type "Float (single-precision)"))
  (if (<= (`self.Health`) 0.0)
    (`self.K2_DestroyActor`)))

(event `TakeDamage`
  (params (damage :type "Float (double-precision)"))
  (`/Engine/EditorBlueprintResources/ActorMacros.Switch Has Authority`
    (:`Authority`
      _)
    (:`Remote`
      _))
  (`self.ApplyDamage` damage))

(fn `ApplyDamage`
  (params (Damage :type "Float (double-precision)"))
  (set `self.Health` (- (`self.Health`) Damage)))

(fn `UserConstructionScript`)